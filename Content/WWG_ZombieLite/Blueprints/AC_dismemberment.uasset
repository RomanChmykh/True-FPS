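; Actor component that handles per-limb damage and dismemberment for skeletal mesh characters in the ZombieLite kit.
; FnOwnerDamaged finds the hit mesh by bone-name component tag, then subtracts damage from the DismembermentStruct entry containing that trigger bone.
; At zero health it swaps in a replacement mesh and breaks a constraint on the first component.
; Otherwise it can simulate trauma physics, applying damage-scaled impulses and blood effects.
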(event EventBeginPlay)

(fn FnFindOwnerMeshComponenttoDismember
  (params (Tag :type Name%20%28by%20ref%29) (DismemberableComponents :type Array%20of%20Skeletal%20Mesh%20Component%20Object%20References))
  (bind _array_element (Utilities|Array|ForEachLoopwithBreak DismemberableComponents :!label _label)
    (:LoopBody
      (LocalVariables|SetComponentHit _array_element)
      (if (Utilities|Array|ContainsItem (Variables|/Script/Engine.ActorComponent|GetComponentTags (LocalVariables|GetComponentHit)) Tag)
        (goto _label Break)))
    (:Completed
      (if (Utilities|Array|ContainsItem (Variables|/Script/Engine.ActorComponent|GetComponentTags (LocalVariables|GetComponentHit)) Tag)
        (return (LocalVariables|GetComponentHit))
        (else
          (return 0))))))

(fn FnFindBodyParttoReplace
  (params (BoneName :type Name) (Damage :type Float%20%28single-precision%29))
  (LocalVariables|SetBoneHit BoneName)
  ;[1 1 1] Breaks loop if trigger bone was hit
  (bind _array_index (Utilities|Array|ForEachLoopwithBreak (Variables|Settings|GetDismembermentStruct) :!label _label)
    (:LoopBody
      (LocalVariables|SetCurrentIndex _array_index)
      (LocalVariables|SetbWasFound? (Utilities|Array|ContainsItem (.TriggerBones (Utilities|Struct|BreakF_Dismemberment (Utilities|Array|Get(acopy) (Variables|Settings|GetDismembermentStruct) (LocalVariables|GetCurrentIndex)))) (LocalVariables|GetBoneHit)))
      (LocalVariables|SetbWasAlreadyDismembered (<= (.Health (Utilities|Struct|BreakF_Dismemberment (Utilities|Array|Get(acopy) (Variables|Settings|GetDismembermentStruct) (LocalVariables|GetCurrentIndex)))) 0.0))
      (if (LocalVariables|GetbWasFound?)
        (goto _label Break)))
    (:Completed
      (if (LocalVariables|GetbWasFound?)
        ;[1 1 1] Set current limb health
        (LocalVariables|SetCurrentHelth (- (.Health (Utilities|Struct|BreakF_Dismemberment (Utilities|Array|Get(acopy) (Variables|Settings|GetDismembermentStruct) (LocalVariables|GetCurrentIndex)))) Damage))
        (Utilities|Array|SetArrayElem (Variables|Settings|GetDismembermentStruct) (LocalVariables|GetCurrentIndex) (Utilities|Struct|MakeF_Dismemberment (.ReplaceBodySkMesh (Utilities|Struct|BreakF_Dismemberment (Utilities|Array|Get(acopy) (Variables|Settings|GetDismembermentStruct) (LocalVariables|GetCurrentIndex)))) (.TriggerBones (Utilities|Struct|BreakF_Dismemberment (Utilities|Array|Get(acopy) (Variables|Settings|GetDismembermentStruct) (LocalVariables|GetCurrentIndex)))) (LocalVariables|GetCurrentHelth) (.ConstraintToBreak (Utilities|Struct|BreakF_Dismemberment (Utilities|Array|Get(acopy) (Variables|Settings|GetDismembermentStruct) (LocalVariables|GetCurrentIndex)))) (.BreakHelth (Utilities|Struct|BreakF_Dismemberment (Utilities|Array|Get(acopy) (Variables|Settings|GetDismembermentStruct) (LocalVariables|GetCurrentIndex)))) (.ShouldTraumaBeSimulated (Utilities|Struct|BreakF_Dismemberment (Utilities|Array|Get(acopy) (Variables|Settings|GetDismembermentStruct) (LocalVariables|GetCurrentIndex))))) true)
        ;[1 1 1] Returns Replace Skeletal and Constraint to Break
        (return (.ReplaceBodySkMesh (Utilities|Struct|BreakF_Dismemberment (Utilities|Array|Get(acopy) (Variables|Settings|GetDismembermentStruct) (LocalVariables|GetCurrentIndex)))) (.ConstraintToBreak (Utilities|Struct|BreakF_Dismemberment (Utilities|Array|Get(acopy) (Variables|Settings|GetDismembermentStruct) (LocalVariables|GetCurrentIndex)))) (and (not (LocalVariables|GetbWasAlreadyDismembered)) (<= (LocalVariables|GetCurrentHelth) 0.0)) (and (not (LocalVariables|GetbWasAlreadyDismembered)) (<= (LocalVariables|GetCurrentHelth) (.BreakHelth (Utilities|Struct|BreakF_Dismemberment (Utilities|Array|Get(acopy) (Variables|Settings|GetDismembermentStruct) (LocalVariables|GetCurrentIndex)))))) (.ShouldTraumaBeSimulated (Utilities|Struct|BreakF_Dismemberment (Utilities|Array|Get(acopy) (Variables|Settings|GetDismembermentStruct) (LocalVariables|GetCurrentIndex)))))
        (else
          (return 0 "None" false false (.ShouldTraumaBeSimulated (Utilities|Struct|BreakF_Dismemberment (Utilities|Array|Get(acopy) (Variables|Settings|GetDismembermentStruct) (LocalVariables|GetCurrentIndex))))))))))

(fn FnOwnerDamaged
  (params (DismemberableComponents :type Array%20of%20Skeletal%20Mesh%20Component%20Object%20References) (Damage :type Float%20%28single-precision%29) (Hit :type Hit%20Result%20Structure))
  (bind (_bblockinghit _binitialoverlap _time _distance _location _impactpoint _normal _impactnormal _physmat _hitactor _hitcomponent _hitbonename _hititem _faceindex _tracestart) (Collision|BreakHitResult Hit))
  (bind _output (Utilities|Array|Get(acopy) DismemberableComponents))
  (bind _output_2 (Utilities|Array|Get(acopy) DismemberableComponents))
  (bind _returnvalue (Math|Vector|Normalize _tracestart))
  (LocalVariables|SetImpilsePower (* (Math|Float|MapRangeClamped Damage 0.0 (Variables|Settings|GetMaxDamage) 0.0 (Variables|Settings|GetMaxImpulse)) -1.0)) ; impulse power mapped to damaged size
  (bind _array_element (CallFunction|FnFindOwnerMeshComponenttoDismember _hitbonename DismemberableComponents)) ; This function finds which skeletal component was hit based on component tags
  (LocalVariables|SetComponentHit _array_element)
  (Utilities|IsValid (LocalVariables|GetComponentHit)
    (:Is%20Valid
      (bind (_replacebodyskmesh _constrainttobreak _bisshouldbedismembered _shouldbebroken _shouldtraumabesimulated) (CallFunction|FnFindBodyParttoReplace _hitbonename Damage)) ; This function chooses replace skeletal mesh instead of full skeletal mesh if its health equal orlower then  0
      (if _bisshouldbedismembered
        (Class|SkinnedMeshComponent|SetSkeletalMesh (LocalVariables|GetComponentHit) _replacebodyskmesh false) ; This function replaces original skeletal mesh to damaged
        (Class|SkeletalMeshComponent|SetAllBodiesBelowSimulatePhysics _output _constrainttobreak true false)
        (Class|SkeletalMeshComponent|BreakConstraint _output (+ _tracestart (Math|Vector|MakeVector (* (.x _returnvalue) (LocalVariables|GetImpilsePower)) (* (.y _returnvalue) (LocalVariables|GetImpilsePower)) (.z _returnvalue))) _location _constrainttobreak)
        (Niagara|SpawnSystematLocation "/Game/WWG_ZombieLite/Particles/NS_BloodBurstBig.NS_BloodBurstBig" _location "0, 0, 0" "1.000000,1.000000,1.000000" true true "AutoRelease")
        (return _bisshouldbedismembered _constrainttobreak (LocalVariables|GetComponentHit) _shouldbebroken)
        (else
          (if (and _shouldbebroken _shouldtraumabesimulated)
            (Class|SkeletalMeshComponent|SetAllBodiesBelowSimulatePhysics _output_2 _hitbonename true true))
          (if (Physics|IsSimulatingPhysics _output_2 _hitbonename)
            (Physics|AddImpulseatLocation _output_2 (+ _tracestart (Math|Vector|MakeVector (* (.x _returnvalue) (LocalVariables|GetImpilsePower)) (* (.y _returnvalue) (LocalVariables|GetImpilsePower)) (.z _returnvalue))) _location _hitbonename)))))
    (:Is%20Not%20Valid
      _))
  (Niagara|SpawnSystematLocation "/Game/WWG_ZombieLite/Particles/NS_BloodBurstSmall.NS_BloodBurstSmall" _location "0, 0, 0" "1.000000,1.000000,1.000000" true true "AutoRelease")
  (return false "None" (select (Utilities|IsValid (LocalVariables|GetComponentHit)) (LocalVariables|GetComponentHit) 0) _shouldbebroken))