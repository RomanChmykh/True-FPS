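; BP_ZombieLite is a zombie character with per-limb dismemberment that chases player-controlled pawns it sees.
; Point damage goes through ACDismemberment, which returns the hit part and break/sever results for head and limb flags; torso hits are unhandled.
; Leg injuries slow walking, more with broken arms, while head loss or four disabled limbs triggers ragdoll.
; Body parts follow the main mesh pose, and a Tick-fed gate reissues AIMoveTo.
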(event OnSeePawn(PawnSensing)
  (params (Pawn :type Pawn%20Object%20Reference))
  ;[1 1 1] FollowPlayer
  (if (and (Pawn|IsPlayerControlled Pawn) (not (CallFunction|FnDeadCheacker)))
    (Utilities|FlowControl|Gate true) ; enters at Open
    (else
      (Utilities|FlowControl|Gate true) ; enters at Close
    )))

(event Game|Damage|EventPointDamage
  (params (Damage :type Float%20%28single-precision%29) (DamageType :type Damage%20Type%20Object%20Reference) (HitLocation :type Vector :default "0, 0, 0") (HitNormal :type Vector :default "0, 0, 0") (HitComponent :type Primitive%20Component%20Object%20Reference) (BoneName :type Name :default "None") (ShotFromDirection :type Vector :default "0, 0, 0") (InstigatedBy :type Controller%20Object%20Reference) (DamageCauser :type Actor%20Object%20Reference) (HitInfo :type Hit%20Result%20Structure%20%28by%20ref%29))
  (bind _dismemberablecomponents (Variables|Default|GetDismemberableComponents))
  ;[1 1 1] Damage
  (bind (_bisshouldbedismembered _constrainttobreak _damagedcomponent _isshouldbebroken) (Default|FnOwnerDamaged (Variables|Default|GetAC_dismemberment) _dismemberablecomponents Damage HitInfo))
  (Utilities|IsValid _damagedcomponent
    (:Is%20Valid
      (switch int (Utilities|Array|FindItem _dismemberablecomponents _damagedcomponent)
        (:1
          (CallFunction|FnHeadDamaged _bisshouldbedismembered HitInfo))
        (:2
          (CallFunction|FnRArmDamaged _isshouldbebroken _bisshouldbedismembered HitInfo))
        (:3
          (CallFunction|FnLArmDamaged _isshouldbebroken _bisshouldbedismembered HitInfo))
        (:4
          (CallFunction|FnRLegDamaged _bisshouldbedismembered _isshouldbebroken HitInfo))
        (:5
          (CallFunction|FnLLegDamaged _isshouldbebroken _bisshouldbedismembered HitInfo)))
      (CallFunction|FnMaxSpeed)
      (if (CallFunction|FnDeadCheacker)
        (Class|SkeletalMeshComponent|SetAllBodiesSimulatePhysics (Variables|Character|GetMesh) true)
        (Collision|SetCollisionEnabled (Variables|Collision|GetCapsuleComponent) "NoCollision")))))

(event EventTick
  (params (DeltaSeconds :type Float%20%28single-precision%29))
  ;[1 1 1] FollowPlayer
  (Utilities|FlowControl|Gate true
    (:Exit
      (AI|AIMoveTo self "0, 0, 0" (stale OnSeePawn(PawnSensing) Pawn) 5.0 false))))

(fn ConstructionScript
  (bind _dismemberablecomponents (Variables|Default|GetDismemberableComponents))
  ;[1 1 1] SynchronizingBodyparts
  (Components|SkinnedMesh|SetLeaderPoseComponent (Variables|Default|GetRArm) (Variables|Character|GetMesh) false false)
  ;[1 1 1] Populating DismemberableComponents Array with components that can be dismembered in game
  (Utilities|Array|Clear _dismemberablecomponents)
  (Utilities|Array|AddUnique _dismemberablecomponents (Variables|Character|GetMesh))
  (Utilities|Array|AddUnique _dismemberablecomponents (Variables|Default|GetHead))
  (Utilities|Array|AddUnique _dismemberablecomponents (Variables|Default|GetRArm))
  (Utilities|Array|AddUnique _dismemberablecomponents (Variables|Default|GetLArm))
  (Utilities|Array|AddUnique _dismemberablecomponents (Variables|Default|GetRLeg))
  (Utilities|Array|AddUnique _dismemberablecomponents (Variables|Default|GetLLeg)))

(fn FnDeadCheacker
  (return (Math|Boolean|ORBoolean (Variables|Default|GetbIsHeadDismembered?) (Variables|Default|GetbIsBodyDismembered?) (Math|Boolean|ANDBoolean (or (Variables|Default|GetbIsLArmDamaged?) (Variables|Default|GetbIsLArmDismembered?)) (or (Variables|Default|GetbIsRArmDamaged?) (Variables|Default|GetbIsRArmDismembered?)) (or (Variables|Default|GetbIsRLegDamaged?) (Variables|Default|GetbIsRLegDismembered)) (or (Variables|Default|GetbIsLLegDamaged?) (Variables|Default|GetbIsLLegDismembered))))))

(fn FnMaxSpeed
  (if (Math|Boolean|ORBoolean (Variables|Default|GetbIsRLegDismembered) (Variables|Default|GetbIsLLegDismembered) (Variables|Default|GetbIsRLegDamaged?) (Variables|Default|GetbIsLLegDamaged?))
    (if (or (Variables|Default|GetbIsRArmDamaged?) (Variables|Default|GetbIsLArmDamaged?))
      (Variables|/Script/Engine.CharacterMovementComponent|SetMaxWalkSpeed (Variables|Character|GetCharacterMovement) 75.0)
      (else
        (Variables|/Script/Engine.CharacterMovementComponent|SetMaxWalkSpeed (Variables|Character|GetCharacterMovement) 1.2e+02)))))

(fn FnBodyDamaged
  (params (bIsBodyDismembered? :type Boolean) (Hit :type Hit%20Result%20Structure))
  (Variables|Default|SetbIsBodyDismembered? bIsBodyDismembered?))

(fn FnHeadDamaged
  (params (bIsHeadDismembered? :type Boolean) (Hit :type Hit%20Result%20Structure))
  (Variables|Default|SetbIsHeadDismembered? bIsHeadDismembered?))

(fn FnRArmDamaged
  (params (bIsRArmDamaged? :type Boolean) (bIsRArmDismembered? :type Boolean) (Hit :type Hit%20Result%20Structure))
  (Variables|Default|SetbIsRArmDamaged? bIsRArmDamaged?)
  (Variables|Default|SetbIsRArmDismembered? bIsRArmDismembered?))

(fn FnLArmDamaged
  (params (bIsLArmDamaged? :type Boolean) (bIsLArmDismembered? :type Boolean) (Hit :type Hit%20Result%20Structure))
  (Variables|Default|SetbIsLArmDamaged? bIsLArmDamaged?)
  (Variables|Default|SetbIsLArmDismembered? bIsLArmDismembered?))

(fn FnRLegDamaged
  (params (bIsRLegDismembered :type Boolean) (bIsRLegDamaged? :type Boolean) (Hit :type Hit%20Result%20Structure))
  (Variables|Default|SetbIsRLegDamaged? bIsRLegDamaged?)
  (Variables|Default|SetbIsRLegDismembered bIsRLegDismembered))

(fn FnLLegDamaged
  (params (bIsLLegDamaged? :type Boolean) (bIsLLegDismembered :type Boolean) (Hit :type Hit%20Result%20Structure))
  (Variables|Default|SetbIsLLegDamaged? bIsLLegDamaged?)
  (Variables|Default|SetbIsLLegDismembered bIsLLegDismembered))